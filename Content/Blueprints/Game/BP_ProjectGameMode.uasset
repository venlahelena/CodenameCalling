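; Game mode that starts the detective game's opening office quest and manages its on-screen quest tracker.
; BeginPlay creates the quest widget and a QuestBase object with two hardcoded item objectives, then adds one objective widget per entry to a vertical box.
; UpdateObjective and HideObjective match row widgets by objective ID to refresh text or remove the row.
; HideQuest removes only the objectives box, leaving the name and description panel.
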(event `self.ReceiveBeginPlay`
  (bind _currentquest (`self.CurrentQuest`))
  (bind _currentquest_2 (`self.CurrentQuest`))
  (bind _wbp_questinformation (`/Game/GUI/Quest/WBP_Quest.WBP_QuestInformation` (`self.QuestWidget`)))
  (bind _returnvalue (`|CreateWidget` "/Game/GUI/Quest/WBP_Quest.WBP_Quest_C" (`GameplayStatics.GetPlayerController` 0)))
  (bind _output_get (set `self.QuestWidget` _returnvalue))
  (`UserWidget.AddToViewport` _output_get 0)
  (bind _returnvalue_2 (`|GenericCreateObject` self "/Script/Calling.QuestBase"))
  (bind _output_get_2 (set `self.CurrentQuest` _returnvalue_2))
  (`QuestBase.SetNumberOfObjectives` _output_get_2 2)
  (`QuestBase.SetQuestDetails` _currentquest "Welcome Detective 13" "Look around the office")
  (`QuestBase.SetQuestObjectives` _currentquest 0 null "/Game/Blueprints/Items/ReadableItem/BP_InvitationLetter.BP_InvitationLetter_C" "Read" "Item" 1)
  (`QuestBase.SetQuestObjectives` _currentquest 1 null "/Game/Blueprints/Items/InsectableItem/BP_InspectableItem.BP_InspectableItem_C" "Open" "Puzzle box" 1)
  (`/Game/GUI/Quest/WBP_QuestInformation.SetQuestName` _wbp_questinformation (`KismetTextLibrary.Conv_StringToText` (`QuestBase.QuestName` _currentquest_2)))
  (`/Game/GUI/Quest/WBP_QuestInformation.SetQuestDescription` _wbp_questinformation (`KismetTextLibrary.Conv_StringToText` (`QuestBase.QuestDescription` _currentquest_2)))
  (`Widget.SetVisibility` _wbp_questinformation "Visible")
  (for _array_element (`QuestBase.QuestObjectives` (`self.CurrentQuest`))
    (bind _returnvalue_3 (`|CreateWidget` "/Game/GUI/Quest/WBP_QuestObjectiveInfromation.WBP_QuestObjectiveInfromation_C"))
    (bind (_clearingtype _enemytoslay _itemtocollect _objectivedescription _objectiveid) (break `QuestObjective` _array_element))
    (`/Game/GUI/Quest/WBP_QuestObjectiveInfromation.SetObjectiveID` _returnvalue_3 _objectiveid)
    (`/Game/GUI/Quest/WBP_QuestObjectiveInfromation.SetObjectiveDescription` _returnvalue_3 (`KismetTextLibrary.Conv_StringToText` _objectivedescription))
    (`VerticalBox.AddChildToVerticalBox` (`/Game/GUI/Quest/WBP_Quest.ObjectivesVerticalBox` (`self.QuestWidget`)) _returnvalue_3)))

(event `self.UpdateObjective`
  (params (ObjectiveNumber :type Integer))
  (for _array_element (`PanelWidget.GetAllChildren` (`/Game/GUI/Quest/WBP_Quest.ObjectivesVerticalBox` (`self.QuestWidget`)))
    (bind _aswbp_quest_objective_infromation (cast `/Game/GUI/Quest/WBP_QuestObjectiveInfromation` _array_element))
    (if (== (`/Game/GUI/Quest/WBP_QuestObjectiveInfromation.ObjectiveID` _aswbp_quest_objective_infromation) ObjectiveNumber)
      (`/Game/GUI/Quest/WBP_QuestObjectiveInfromation.SetObjectiveDescription` _aswbp_quest_objective_infromation (`KismetTextLibrary.Conv_StringToText` (`.ObjectiveDescription` (break `QuestObjective` (`|GetArrayItem` (`QuestBase.QuestObjectives` (`self.CurrentQuest`)) ObjectiveNumber))))))))

(event `self.HideObjective`
  (params (ObjectiveNumber :type Integer))
  (bind _objectivesverticalbox (`/Game/GUI/Quest/WBP_Quest.ObjectivesVerticalBox` (`self.QuestWidget`)))
  (for _array_element (`PanelWidget.GetAllChildren` _objectivesverticalbox)
    (bind _aswbp_quest_objective_infromation (cast `/Game/GUI/Quest/WBP_QuestObjectiveInfromation` _array_element))
    (if (== (`/Game/GUI/Quest/WBP_QuestObjectiveInfromation.ObjectiveID` _aswbp_quest_objective_infromation) ObjectiveNumber)
      (`PanelWidget.RemoveChild` _objectivesverticalbox _aswbp_quest_objective_infromation))))

(event `self.HideQuest`
  (`Widget.RemoveFromParent` (`/Game/GUI/Quest/WBP_Quest.ObjectivesVerticalBox` (`self.QuestWidget`))))

(fn `UserConstructionScript`)