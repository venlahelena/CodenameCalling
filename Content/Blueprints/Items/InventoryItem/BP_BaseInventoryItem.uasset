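; Base inventory item Blueprint that reports its own collection to the quest system.
; NotifyCollectedforQuest gets the current quest from BP_ProjectGameMode and loops through its objectives.
; When the item's class is a child of, and exactly equal to, an objective's ItemToCollect, it calls UpdateObjectives with that objective's ID and a value of one.
; The exact-equality check means subclasses of the requested item do not count.
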(event `self.NotifyCollectedForQuest`
  (bind _returnvalue (`GameplayStatics.GetObjectClass` self))
  (bind _asbp_project_game_mode (cast `/Game/Blueprints/Game/BP_ProjectGameMode` (`GameplayStatics.GetGameMode`)))
  (bind _currentquest (`/Game/Blueprints/Game/BP_ProjectGameMode.CurrentQuest` _asbp_project_game_mode))
  (for _array_element (`QuestBase.QuestObjectives` _currentquest)
    (bind (_clearingtype _enemytoslay _itemtocollect _objectivedescription _objectiveid) (break `QuestObjective` _array_element))
    (if (`KismetMathLibrary.ClassIsChildOf` _returnvalue _itemtocollect)
      (if (== _returnvalue _itemtocollect)
        (`QuestBase.UpdateObjectives` _currentquest _objectiveid 1)))))

(fn `UserConstructionScript`)